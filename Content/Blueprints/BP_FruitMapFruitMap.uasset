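; BP_FruitMapFruitMap is a Blueprint that lays out the standard Map container nodes on a FruitMap of integer keys and fruit-name strings.
; Its EventGraph holds unconnected examples of building, editing and querying the map, with lookups and removals tried on two different keys.
; None of these nodes run: BeginPlay and the construction script are empty, so the asset has no runtime behavior.
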(fn `UserConstructionScript`)