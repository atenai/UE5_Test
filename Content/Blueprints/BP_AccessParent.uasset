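; BP_AccessParent is a demo parent Blueprint for function and variable access levels, named as public, protected and private.
; CallPublicFunc, CallProtectedFunc and CallPrivateFunc each print the object's display name, the function name and their matching number variable in a distinct, long-lasting color.
; The event graph holds calls to all three, but none is wired to an event, so this Blueprint never runs them itself.
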(event `self.ReceiveBeginPlay`)

(fn `CallPrivateFunc`
  (`KismetSystemLibrary.PrintString` (`KismetStringLibrary.Concat_StrStr` (`KismetSystemLibrary.GetDisplayName` self) " : CallPrivateFunc" (`KismetStringLibrary.Conv_IntToString` (`self.VarPrivateNum`))) true true (struct :`R` 0.384813 :`B` 1.0 :`A` 1.0) 100.0))

(fn `CallProtectedFunc`
  (`KismetSystemLibrary.PrintString` (`KismetStringLibrary.Concat_StrStr` (`KismetSystemLibrary.GetDisplayName` self) " : CallProtectedFunc" (`KismetStringLibrary.Conv_IntToString` (`self.VarProtectedNum`))) true true (struct :`R` 1.0 :`B` 0.950316 :`A` 1.0) 100.0))

(fn `CallPublicFunc`
  (`KismetSystemLibrary.PrintString` (`KismetStringLibrary.Concat_StrStr` (`KismetSystemLibrary.GetDisplayName` self) " : CallPublicFunc" (`KismetStringLibrary.Conv_IntToString` (`self.VarPublicNum`))) true true (struct :`R` 1.0 :`B` 0.126024 :`A` 1.0) 100.0))

(fn `UserConstructionScript`)