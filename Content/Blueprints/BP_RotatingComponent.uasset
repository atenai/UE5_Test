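; BP_RotatingComponent is a component that continuously rotates its owning actor by fixed increments at a set interval.
; On BeginPlay it caches the owner root component's world rotation and starts a looping timer instead of using Tick.
; Each timer call adds per-axis offsets to the cached rotation and applies it to the root, overriding any rotation changes made elsewhere.
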(event `self.ReceiveBeginPlay`
  (set `self.OwnerRotation` (`SceneComponent.K2_GetComponentRotation` (`Actor.RootComponent` (`self.GetOwner`))))
  (`KismetSystemLibrary.K2_SetTimerDelegate` (delegate `Rotate`) (`self.Interval`) true))

(event `Rotate`
  (bind (_ownerrotation_roll _ownerrotation_pitch _ownerrotation_yaw) (`KismetMathLibrary.BreakRotator` (`self.OwnerRotation`)))
  (bind _output_get (set `self.OwnerRotation` (`KismetMathLibrary.MakeRotator` (+ _ownerrotation_roll (`self.Rot(X)`)) (+ _ownerrotation_pitch (`self.Rot(Y)`)) (+ _ownerrotation_yaw (`self.Rot(Z)`)))))
  (`SceneComponent.K2_SetWorldRotation` (`Actor.RootComponent` (`self.GetOwner`)) _output_get false false))