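; BP_EnhancedInputTest is a test Blueprint that exercises Enhanced Input and prints the results.
; On BeginPlay it enables input from player controller 0 and adds IMC_Default to that player's Enhanced Input subsystem.
; IA_Action prints "Pressed" once per press through a DoOnce gate, which Completed resets while printing "Released".
; IA_Axis prints its X and Y values whenever it triggers.
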(event `self.ReceiveBeginPlay`
  (bind _returnvalue (`GameplayStatics.GetPlayerController` 0))
  (bind _returnvalue_2 (pcsubsystem `EnhancedInputLocalPlayerSubsystem` _returnvalue))
  (`|ExecutionSequence`
    (:`then_0`
      (`self.EnableInput` _returnvalue))
    (:`then_1`
      (`/Engine/EditorBlueprintResources/StandardMacros.IsValid` _returnvalue_2
        (:`Is Valid`
          (`EnhancedInputSubsystemInterface.AddMappingContext` _returnvalue_2 "/Game/Input/IMC_Default.IMC_Default" 0 (struct)))))))

(event `EnhancedInput|/Game/Input/Actions/IA_Action`
  (params (ActionValue :type Boolean) (ElapsedSeconds :type "Float (double-precision)") (TriggeredSeconds :type "Float (double-precision)") (InputAction :type "InputAction Object Reference" :default "/Game/Input/Actions/IA_Action.IA_Action"))
  (:`Triggered`
    (`/Engine/EditorBlueprintResources/StandardMacros.DoOnce` false :!label _label
      (:`Completed`
        (`KismetSystemLibrary.PrintString` "Pressed" true true (struct :`R` 1.0 :`G` 0.174571 :`A` 1.0) 20.0))))
  (:`Completed`
    (`|ExecutionSequence`
      (:`then_0`
        (goto _label :!via `Reset`))
      (:`then_1`
        (`KismetSystemLibrary.PrintString` "Released" true true (struct :`G` 1.0 :`B` 0.256161 :`A` 1.0) 20.0)))))

(event `EnhancedInput|/Game/Input/Actions/IA_Axis`
  (params (ActionValue :type "Vector2D Structure") (ElapsedSeconds :type "Float (double-precision)") (TriggeredSeconds :type "Float (double-precision)") (InputAction :type "InputAction Object Reference" :default "/Game/Input/Actions/IA_Axis.IA_Axis"))
  (bind (_x _y) (`KismetMathLibrary.BreakVector2D` ActionValue))
  (:`Triggered`
    (`KismetSystemLibrary.PrintString` (`KismetStringLibrary.Concat_StrStr` "X : " (`KismetStringLibrary.Conv_DoubleToString` _x) "Y : " (`KismetStringLibrary.Conv_DoubleToString` _y)) true true (struct :`G` 1.0 :`B` 0.256161 :`A` 1.0) 20.0)))

(fn `UserConstructionScript`)