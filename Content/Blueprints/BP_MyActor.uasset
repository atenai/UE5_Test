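; BP_MyActor is a skeleton Blueprint with no active runtime behavior, as its BeginPlay and Tick events are empty.
; The construction script resets MemberVar to zero, while disconnected nodes hold logic to accumulate delta time into it and print it in green, plus a DistanceFromActor call.
; A standalone Func sums two inputs through a local variable and returns half and double that sum, with no caller in the graphs.
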(event `self.ReceiveTick`
  (params (DeltaSeconds :type "Float (single-precision)")))

(fn `Func`
  (params (In1 :type "Float (double-precision)") (In2 :type "Float (double-precision)"))
  (returns (Out1 :type "Float (double-precision)") (Out2 :type "Float (double-precision)"))
  (bind _output_get (set `self.LocalVar` (+ In1 In2)))
  (return (/ _output_get 2.0) (* _output_get 2.0)))

(fn `UserConstructionScript`
  (set `self.MemberVar` 0.0))