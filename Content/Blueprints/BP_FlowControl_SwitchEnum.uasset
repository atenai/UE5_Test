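; BP_FlowControl_SwitchEnum is a flow-control practice actor that prints a message or a calculation result on BeginPlay.
; When IsPrintHello is false, a switch on the CPPCalcType enum selects addition, subtraction, multiplication or division of CalcVarA and CalcVarB, printed in distinct colours.
; The construction script sets the PointLight's visibility, intensity and colour from variables.
; Disconnected alternative branches (int switch, CalcType enum, if chain, sequence) remain but never run.
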(event EventBeginPlay
  (if (Variables|FlowControl|GetIsPrintHello)
    ;[0.5512 0.8369 1] コメントボックス
    (Development|PrintString (Variables|PrintString|GetMessage) true true (Variables|PrintString|GetTextColor) (Variables|PrintString|GetDuration)) ; BP_HelloWorldと表示する
    (else
      (switch Utilities|FlowControl|Switch|SwitchonECPPCalcType (Variables|FlowControl|GetCPPCalcType)
        (:Add
          ;[1 0 0.03535] 足し算
          (Development|PrintString (Utilities|String|ToString(Float) (|(A+B) (Math|Conversions|ToFloat(Integer) (Variables|Calculation|GetCalcVarA)) (Math|Conversions|ToFloat(Integer) (Variables|Calculation|GetCalcVarB)))) true true "(R=1.000000,G=0.000000,B=0.100150,A=1.000000)" (Variables|PrintString|GetDuration)) ; BP_HelloWorldと表示する
        )
        (:Subtract
          ;[0.1423 0 1] 引き算
          (Development|PrintString (Utilities|String|ToString(Integer) (- (Variables|Calculation|GetCalcVarA) (Variables|Calculation|GetCalcVarB))) true true "(R=0.115812,G=0.000000,B=1.000000,A=1.000000)" (Variables|PrintString|GetDuration)) ; BP_HelloWorldと表示する
        )
        (:Multiply
          ;[1 0.8671 0] 掛け算
          (Development|PrintString (Utilities|String|ToString(Integer) (* (Variables|Calculation|GetCalcVarA) (Variables|Calculation|GetCalcVarB))) true true "(R=1.000000,G=0.860987,B=0.000000,A=1.000000)" (Variables|PrintString|GetDuration)) ; BP_HelloWorldと表示する
        )
        (:Divide
          ;[0 1 0.5013] 割り算
          (Development|PrintString (Utilities|String|ToString(Float) (/ (Variables|Calculation|GetCalcVarA) (Variables|Calculation|GetCalcVarB))) true true "(R=0.019283,G=1.000000,B=0.799529,A=1.000000)" (Variables|PrintString|GetDuration)) ; BP_HelloWorldと表示する
        )))))

(event Collision|EventActorBeginOverlap
  (params (OtherActor :type Actor%20Object%20Reference)))

(event EventTick
  (params (DeltaSeconds :type Float%20%28single-precision%29)))

(fn ConstructionScript
  ;[1 1 1] ポイントライトの表示/非表示
  (Rendering|SetVisibility (Variables|Default|GetPointLight) (Variables|PointLight|GetIsVisible) false)
  ;[1 1 1] PointLightのIntensityを設定する
  (Rendering|Components|Light|SetIntensity (Variables|Default|GetPointLight) (Variables|PointLight|GetIntensity))
  ;[1 1 1] PointLightのLightColorを設定する
  (Rendering|Components|Light|SetLightColor (Variables|Default|GetPointLight) (Variables|PointLight|GetLightColor) true))