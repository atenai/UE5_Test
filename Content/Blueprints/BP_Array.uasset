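; BP_Array is a practice actor for Blueprint array operations, printing results on screen.
; BeginPlay swaps two Greetings entries and prints the array, while many other array nodes sit disconnected.
; ActionPrintCalcResult runs the CalcTypes operation at TypeIndex on two variables, then advances the index with modulo wraparound.
; The construction script configures a PointLight; H calls OnPrintHello, but its PrintHello binding and EnableInput are disconnected.
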(event `self.ReceiveBeginPlay`
  (bind _greetings (`self.Greetings`))
  (`KismetArrayLibrary.Array_Swap` _greetings 0 4)
  (for (_array_element _array_index) _greetings
    (`KismetSystemLibrary.PrintString` (`KismetStringLibrary.Concat_StrStr` (`KismetStringLibrary.Conv_IntToString` _array_index) " : " _array_element) true true (struct :`R` 1.0 :`B` 0.106402 :`A` 1.0) 20.0)))

(event `PrintHello`
  (bind _messages (`self.Messages`))
  (bind (_outitem _outindex) (`KismetArrayLibrary.Array_Random` _messages))
  ;[0.5512 0.8369 1] コメントボックス
  (`KismetSystemLibrary.PrintString` (`|GetArrayItem` _messages (`KismetMathLibrary.RandomIntegerInRange` 0 (- (`KismetArrayLibrary.Array_Length` _messages) 1))) true true (`self.TextColor`) (`self.Duration`)) ; BP_HelloWorldと表示する
  (`KismetSystemLibrary.PrintString` _outitem true true (struct :`R` 1.0 :`G` 0.606406 :`A` 1.0)) ; BP_HelloWorldと表示する
  (`KismetSystemLibrary.PrintString` (`|GetArrayItem` _messages _outindex) true true (struct :`R` 1.0 :`G` 0.083189 :`A` 1.0)) ; BP_HelloWorldと表示する
)

(event `Key|H`
  (params (Key :type "Key Structure"))
  (:`Pressed`
    (`self.OnPrintHello`) ; OnPrintHelloを呼び出す
  ))

(event `InputAction|ActionPrintCalcResult`
  (params (Key :type "Key Structure"))
  (bind _returnvalue (mod (`self.TypeIndex`) (`KismetArrayLibrary.Array_Length` (`self.CalcTypes`))))
  (bind _returnvalue_2 (mod (`self.TypeIndex`) (`KismetArrayLibrary.Array_Length` (`self.CalcTypes`))))
  (bind _returnvalue_3 (mod (`self.TypeIndex`) (`KismetArrayLibrary.Array_Length` (`self.CalcTypes`))))
  (bind _returnvalue_4 (mod (`self.TypeIndex`) (`KismetArrayLibrary.Array_Length` (`self.CalcTypes`))))
  (:`Released`
    (switch `/Game/Blueprints/EBPCalcType` (`|GetArrayItem` (`self.CalcTypes`) (`self.TypeIndex`))
      (:`NewEnumerator0`
        ;[1 0 0.03535] 足し算
        (`KismetSystemLibrary.PrintString` (`KismetStringLibrary.Conv_IntToString` (`self.Sum` (`self.CalcVarA`) (`self.CalcVarB`))) true true (struct :`R` 1.0 :`B` 0.10015 :`A` 1.0) (`self.Duration`)) ; BP_HelloWorldと表示する
        (`/Engine/EditorBlueprintResources/StandardMacros.IncrementInt` (`self.TypeIndex`)
          (:`  `
            (set `self.TypeIndex` _returnvalue_2)
            (`KismetSystemLibrary.PrintString` (`KismetStringLibrary.Conv_IntToString` _returnvalue_2) true true (struct :`G` 0.66 :`B` 1.0 :`A` 1.0) 20.0))))
      (:`NewEnumerator1`
        ;[0.1423 0 1] 引き算
        (`KismetSystemLibrary.PrintString` (`KismetStringLibrary.Conv_IntToString` (- (`self.CalcVarA`) (`self.CalcVarB`))) true true (struct :`R` 0.115812 :`B` 1.0 :`A` 1.0) (`self.Duration`)) ; BP_HelloWorldと表示する
        (`/Engine/EditorBlueprintResources/StandardMacros.IncrementInt` (`self.TypeIndex`)
          (:`  `
            (set `self.TypeIndex` _returnvalue)
            (`KismetSystemLibrary.PrintString` (`KismetStringLibrary.Conv_IntToString` _returnvalue) true true (struct :`G` 0.66 :`B` 1.0 :`A` 1.0) 20.0))))
      (:`NewEnumerator2`
        ;[1 0.8671 0] 掛け算
        (`KismetSystemLibrary.PrintString` (`KismetStringLibrary.Conv_IntToString` (* (`self.CalcVarA`) (`self.CalcVarB`))) true true (struct :`R` 1.0 :`G` 0.860987 :`A` 1.0) (`self.Duration`)) ; BP_HelloWorldと表示する
        (`/Engine/EditorBlueprintResources/StandardMacros.IncrementInt` (`self.TypeIndex`)
          (:`  `
            (set `self.TypeIndex` _returnvalue_3)
            (`KismetSystemLibrary.PrintString` (`KismetStringLibrary.Conv_IntToString` _returnvalue_3) true true (struct :`G` 0.66 :`B` 1.0 :`A` 1.0) 20.0))))
      (:`NewEnumerator3`
        ;[0 1 0.5013] 割り算
        (`KismetSystemLibrary.PrintString` (`KismetStringLibrary.Conv_DoubleToString` (/ (`self.CalcVarA`) (`self.CalcVarB`))) true true (struct :`R` 0.019283 :`G` 1.0 :`B` 0.799529 :`A` 1.0) (`self.Duration`)) ; BP_HelloWorldと表示する
        (`/Engine/EditorBlueprintResources/StandardMacros.IncrementInt` (`self.TypeIndex`)
          (:`  `
            (set `self.TypeIndex` _returnvalue_4)
            (`KismetSystemLibrary.PrintString` (`KismetStringLibrary.Conv_IntToString` _returnvalue_4) true true (struct :`G` 0.66 :`B` 1.0 :`A` 1.0) 20.0)))))))

(fn `Sum`
  (params (A :type "Integer (by ref)") (B :type "Integer (by ref)"))
  (returns (ReturnValue :type Integer))
  (locals (LocalResult :type Integer))
  (bind _output_get (set `local.LocalResult` (+ A B)))
  (return _output_get))

(fn `UserConstructionScript`
  ;[1 1 1] ポイントライトの表示/非表示
  (`SceneComponent.SetVisibility` (`self.PointLight`) (`self.IsVisible`) false)
  ;[1 1 1] PointLightのIntensityを設定する
  (`LightComponent.SetIntensity` (`self.PointLight`) (`self.Intensity`))
  ;[1 1 1] PointLightのLightColorを設定する
  (`LightComponent.SetLightColor` (`self.PointLight`) (`self.LightColor`) true))