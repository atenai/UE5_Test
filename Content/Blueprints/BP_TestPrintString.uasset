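; BP_TestPrintString is a test Blueprint for printing values on screen, with no active logic.
; BeginPlay, Tick and the construction script are empty, and the other event graph nodes are disconnected, so they never run.
; These disconnected chains print the result of a simple Sum function, print real time under a fixed key, and store a MakeMoveParam result.
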(event `self.ReceiveBeginPlay`)

(event `self.ReceiveTick`
  (params (DeltaSeconds :type "Float (single-precision)")))

(fn `Sum`
  (params (A :type Integer) (B :type Integer))
  (returns (ReturnValue :type Integer))
  (locals (TotalLocal :type Integer))
  (bind _output_get (set `local.TotalLocal` (+ A B)))
  (return _output_get))

(fn `UserConstructionScript`)