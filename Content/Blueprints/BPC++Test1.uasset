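; Test Blueprint that exercises calls between Blueprint and a C++ actor class, MySomeCPPActor.
; On BeginPlay it finds the BP_MyActor instance in the level, stores it in RefActor and prints its display name.
; It then prints the result of the static C++ function StaticGet2023.
; Finally it locates MySomeCPPActor and passes its truncated Get10 result to that actor's TestPrint.
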(event `self.ReceiveBeginPlay`
  ;[1 1 1] BP_MyActorクラスを取得してクラス型に入れる
  (bind _returnvalue (`GameplayStatics.GetActorOfClass` "/Game/Blueprints/BP_MyActor.BP_MyActor_C"))
  (set `self.RefActor` _returnvalue)
  (`KismetSystemLibrary.PrintString` (`KismetSystemLibrary.GetDisplayName` (`self.RefActor`)) true true (struct :`R` 0.927083 :`G` 1.0 :`B` 1.0 :`A` 1.0) 202.0)
  ;[1 1 1] C++で作成したMySomeCPPActorのStatic関数の呼び出す
  (`KismetSystemLibrary.PrintString` (`KismetStringLibrary.Conv_IntToString` (`MySomeCPPActor.StaticGet2023`)) true true (struct :`R` 1.0 :`B` 0.23525 :`A` 1.0) 202.0)
  ;[1 1 1] C++で作成したMySomeCPPActorの通常の関数を呼び出す
  (bind _returnvalue_2 (`GameplayStatics.GetActorOfClass` "/Script/CPP_BP.MySomeCPPActor"))
  (`MySomeCPPActor.TestPrint` _returnvalue_2 (`KismetMathLibrary.FTrunc` (`MySomeCPPActor.Get10` _returnvalue_2))))

(event `self.ReceiveTick`
  (params (DeltaSeconds :type "Float (single-precision)")))

(fn `UserConstructionScript`)