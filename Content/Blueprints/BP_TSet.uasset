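; BP_TSet is a demo Blueprint for Set container operations on a string set, FruitSet.
; On BeginPlay it prints every element, adds "Orange", removes "Apple", then prints the set again in a different color to show the change.
; Unconnected nodes hold samples of other Set functions, including bulk add and remove, clear, union, intersection, difference and queries, none of which run.
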(event `self.ReceiveBeginPlay`
  (bind _fruitset (`self.FruitSet`))
  (`|ExecutionSequence`
    (:`then_0`
      (bind _result (`BlueprintSetLibrary.Set_ToArray` (`self.FruitSet`)))
      (for _array_element _result
        (`KismetSystemLibrary.PrintString` _array_element true true (struct :`R` 1.0 :`B` 0.513882 :`A` 1.0) 20.0)))
    (:`then_1`
      (`BlueprintSetLibrary.Set_Add` _fruitset "Orange"))
    (:`then_2`
      (`BlueprintSetLibrary.Set_Remove` _fruitset "Apple"))
    (:`then_3`
      (bind _result_2 (`BlueprintSetLibrary.Set_ToArray` (`self.FruitSet`)))
      (for _array_element_2 _result_2
        (`KismetSystemLibrary.PrintString` _array_element_2 true true (struct :`R` 1.0 :`G` 0.126577 :`A` 1.0) 20.0)))))

(fn `UserConstructionScript`)