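; BP_ConstructionScript is an actor Blueprint that demonstrates configuring a PointLight component through its Construction Script.
; The Construction Script sets the light's visibility, intensity and color from the IsVisible, Intensity and LightColor variables.
; On BeginPlay it prints the Message variable to the screen using the TextColor and Duration variables.
; Tick and ActorBeginOverlap are unused.
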(event `self.ReceiveBeginPlay`
  ;[1 0.8086 0] コメントボックス
  (`KismetSystemLibrary.PrintString` (`self.Message`) true true (`self.TextColor`) (`self.Duration`)) ; BP_HelloWorldと表示する
)

(fn `UserConstructionScript`
  ;[1 1 1] ポイントライトの表示/非表示
  (`SceneComponent.SetVisibility` (`self.PointLight`) (`self.IsVisible`) false)
  ;[1 1 1] PointLightのIntensityを設定する
  (`LightComponent.SetIntensity` (`self.PointLight`) (`self.Intensity`))
  ;[1 1 1] PointLightのLightColorを設定する
  (`LightComponent.SetLightColor` (`self.PointLight`) (`self.LightColor`) true))