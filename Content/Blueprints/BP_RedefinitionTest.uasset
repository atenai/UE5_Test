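; BP_RedefinitionTest is a test actor that compares function behavior between a parent Blueprint and its child, apparently to demonstrate overriding.
; On BeginPlay, a sequence spawns BP_ParentRedefinition and then BP_ChildRedefinition at the origin.
; Each instance receives the same SetPoint value, then its GetPoint result prints on screen in a distinct color for comparison.
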(event `self.ReceiveBeginPlay`
  (bind _returnvalue (`KismetMathLibrary.MakeTransform` (0.0 0.0 0.0)))
  (`|ExecutionSequence`
    (:`then_0`
      (bind _returnvalue_2 (`|SpawnActorFromClass` "/Game/Blueprints/BP_ParentRedefinition.BP_ParentRedefinition_C" _returnvalue "Undefined" "OverrideRootScale" null null))
      (`/Game/Blueprints/BP_ParentRedefinition.SetPoint` _returnvalue_2 100)
      (bind _returnvalue_3 (`/Game/Blueprints/BP_ParentRedefinition.GetPoint` _returnvalue_2))
      (`KismetSystemLibrary.PrintString` (`KismetStringLibrary.Concat_StrStr` "Parent Point : " (`KismetStringLibrary.Conv_IntToString` _returnvalue_3)) true true (struct :`G` 0.045144 :`B` 1.0 :`A` 1.0) 10.0))
    (:`then_1`
      (bind _returnvalue_4 (`|SpawnActorFromClass` "/Game/Blueprints/BP_ChildRedefinition.BP_ChildRedefinition_C" _returnvalue "Undefined" "OverrideRootScale" null null))
      (`/Game/Blueprints/BP_ParentRedefinition.SetPoint` _returnvalue_4 100)
      (bind _returnvalue_5 (`/Game/Blueprints/BP_ParentRedefinition.GetPoint` _returnvalue_4))
      (`KismetSystemLibrary.PrintString` (`KismetStringLibrary.Concat_StrStr` "Child Point : " (`KismetStringLibrary.Conv_IntToString` _returnvalue_5)) true true (struct :`R` 1.0 :`B` 0.127908 :`A` 1.0) 10.0))))

(fn `UserConstructionScript`)