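; BP_TMap is a demonstration Blueprint that exercises map container operations on a FruitMap of numeric keys and string values.
; On BeginPlay, a Sequence prints all keys, all values, then key-value pairs by indexing the Values array with the Keys loop index.
; It then looks up a key with Find, adds and removes entries, and reprints the changed map using per-key Find, with colored on-screen text.
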(event `self.ReceiveBeginPlay`
  (bind _fruitmap (`self.FruitMap`))
  (bind _fruitmap_2 (`self.FruitMap`))
  (bind _fruitmap_3 (`self.FruitMap`))
  (bind (_value _returnvalue) (`BlueprintMapLibrary.Map_Find` _fruitmap_3 3))
  (`|ExecutionSequence`
    (:`then_0`
      (bind _keys (`BlueprintMapLibrary.Map_Keys` _fruitmap_2))
      (for _array_element _keys
        (`KismetSystemLibrary.PrintString` (`KismetStringLibrary.Conv_IntToString` _array_element) true true (struct :`R` 1.0 :`B` 0.26867 :`A` 1.0) 20.0)))
    (:`then_1`
      (bind _values (`BlueprintMapLibrary.Map_Values` _fruitmap_2))
      (for _array_element_2 _values
        (`KismetSystemLibrary.PrintString` _array_element_2 true true (struct :`R` 0.487913 :`B` 1.0 :`A` 1.0) 20.0)))
    (:`then_2`
      (bind _values_2 (`BlueprintMapLibrary.Map_Values` _fruitmap_3))
      (bind _keys_2 (`BlueprintMapLibrary.Map_Keys` _fruitmap_3))
      (for (_array_element_3 _array_index) _keys_2
        (`KismetSystemLibrary.PrintString` (`KismetStringLibrary.Concat_StrStr` "Keys : " (`KismetStringLibrary.Conv_IntToString` _array_element_3) " " "Values : " (`|GetArrayItem` _values_2 _array_index)) true true (struct :`R` 1.0 :`G` 0.255102 :`A` 1.0) 20.0)))
    (:`then_3`
      (if _returnvalue
        (`KismetSystemLibrary.PrintString` _value true true (struct :`R` 1.0 :`B` 0.71538 :`A` 1.0) 20.0)))
    (:`then_4`
      (`BlueprintMapLibrary.Map_Add` _fruitmap 12 "Orange")
      (`BlueprintMapLibrary.Map_Remove` _fruitmap 3)
      (bind _keys_3 (`BlueprintMapLibrary.Map_Keys` _fruitmap))
      (for _array_element_4 _keys_3
        (`KismetSystemLibrary.PrintString` (`KismetStringLibrary.Concat_StrStr` "Keys : " (`KismetStringLibrary.Conv_IntToString` _array_element_4) " " "Values : " (`BlueprintMapLibrary.Map_Find` _fruitmap _array_element_4)) true true (struct :`R` 0.966619 :`G` 1.0 :`A` 1.0) 20.0)))))

(fn `UserConstructionScript`)