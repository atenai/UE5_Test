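; Bird Blueprint that uses inherited or externally defined vitality, flight speed, FlightBooster fuel and ID members, with almost no logic of its own.
; The construction script prints BirdID on screen for a long duration, as the only live behavior in these graphs.
; BeginPlay, Tick and overlap events are empty, leaving disconnected debug chains that would test damage and healing or print stats and IDs.
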(event `self.ReceiveBeginPlay`)

(event `self.ReceiveTick`
  (params (DeltaSeconds :type "Float (single-precision)")))

(fn `UserConstructionScript`
  (`KismetSystemLibrary.PrintString` (`KismetStringLibrary.Conv_IntToString` (`self.BirdID`)) true true (struct :`R` 0.368404 :`B` 1.0 :`A` 1.0) 100.0))