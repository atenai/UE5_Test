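; BP_ClassChild is a child Blueprint that exercises class inheritance by using both inherited and local members.
; BeginPlay sets VarParentNum, then calls CallParentFunc and its own CallChildFunc, which prints the object's display name with VarChildNum.
; The parent BeginPlay call is left unwired, so the parent's BeginPlay logic does not run, while the construction script still calls the parent's.
; The overlap and Tick events are disabled placeholders.
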(event `self.ReceiveBeginPlay`
  (set `self.VarParentNum` 2000)
  (`self.CallParentFunc`)
  (`self.CallChildFunc`))

(fn `CallChildFunc`
  (`KismetSystemLibrary.PrintString` (`KismetStringLibrary.Concat_StrStr` (`KismetSystemLibrary.GetDisplayName` self) " : CallChildFunc" (`KismetStringLibrary.Conv_IntToString` (`self.VarChildNum`)))))

(fn `UserConstructionScript`
  (`parent.UserConstructionScript`))