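; BP_BallPlayer is the player-controlled rolling ball, driven by Enhanced Input.
; BeginPlay registers the IM_Controls mapping context with the first player controller's input subsystem.
; IA_Control pushes the Sphere with a mass-independent force, scaled by Speed and oriented by the Arrow component's world transform.
; IA_Look adds yaw and pitch input, then clamps control pitch to keep the camera within a downward-looking range.
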(event `self.ReceiveBeginPlay`
  (bind _returnvalue (pcsubsystem `EnhancedInputLocalPlayerSubsystem` (`GameplayStatics.GetPlayerController` 0)))
  ;[1 1 1] Input方法を「IM_Control」に設定する
  (`/Engine/EditorBlueprintResources/StandardMacros.IsValid` _returnvalue
    (:`Is Valid`
      (`EnhancedInputSubsystemInterface.AddMappingContext` _returnvalue "/Game/RollingBall/Input/IM_Controls.IM_Controls" 0 (struct)))))

(event `EnhancedInput|/Game/RollingBall/Input/Action/IA_Control`
  (params (ActionValue :type "Vector2D Structure") (ElapsedSeconds :type "Float (double-precision)") (TriggeredSeconds :type "Float (double-precision)") (InputAction :type "InputAction Object Reference" :default "/Game/RollingBall/Input/Action/IA_Control.IA_Control"))
  (bind (_x _y) (`KismetMathLibrary.BreakVector2D` ActionValue))
  ;[1 1 1] Sphereに力を加える
  (:`Triggered`
    (`PrimitiveComponent.AddForce` (`self.Sphere`) (* (`KismetMathLibrary.TransformDirection` (`SceneComponent.K2_GetComponentToWorld` (`self.Arrow`)) (`KismetMathLibrary.MakeVector` _y _x)) (`self.Speed`)) "None" true)))

(event `EnhancedInput|/Game/RollingBall/Input/Action/IA_Look`
  (params (ActionValue :type "Vector2D Structure") (ElapsedSeconds :type "Float (double-precision)") (TriggeredSeconds :type "Float (double-precision)") (InputAction :type "InputAction Object Reference" :default "/Game/RollingBall/Input/Action/IA_Look.IA_Look"))
  (bind (_x _y) (`KismetMathLibrary.BreakVector2D` ActionValue))
  ;[1 1 1] コントローラーの角度を変更する
  (:`Triggered`
    (`|ExecutionSequence`
      (:`then_0`
        (`self.AddControllerYawInput` _x)
        (`self.AddControllerPitchInput` _y))
      (:`then_1`
        ;[1 1 1] カメラの操作を制限する
        (`Controller.SetControlRotation` (`GameplayStatics.GetPlayerController` 0) (`KismetMathLibrary.MakeRotator` 0.0 (`KismetMathLibrary.ClampAngle` (.pitch (`self.GetControlRotation`)) -40.0 -10.0) (.yaw (`self.GetControlRotation`))))))))

(fn `UserConstructionScript`)