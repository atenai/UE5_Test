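; BP_Heart is a heart item in the RollingBall game that heals the player's ball.
; GetItem casts the first player pawn to BP_BallPlayer, calls Heal with HealValue, and prints the result on screen as debug text.
; Its own event graph holds only disabled placeholder events, so nothing in this Blueprint calls GetItem.
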(fn `GetItem`
  (bind _asbp_ball_player (cast `/Game/RollingBall/Blueprint/Character/BP_BallPlayer` (`GameplayStatics.GetPlayerPawn` 0)))
  (bind _returnvalue (`/Game/RollingBall/Blueprint/Character/BP_BallPlayer.Heal` _asbp_ball_player (`self.HealValue`)))
  (`KismetSystemLibrary.PrintString` (`KismetStringLibrary.Conv_DoubleToString` _returnvalue) true true (struct :`R` 1.0 :`B` 0.785793 :`A` 1.0) 10.0))

(fn `UserConstructionScript`
  (`parent.UserConstructionScript`))