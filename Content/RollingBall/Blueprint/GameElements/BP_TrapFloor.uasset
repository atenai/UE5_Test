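; BP_TrapFloor is a trap floor for the rolling ball game that knocks back and damages the player ball on contact.
; When a BP_BallPlayer overlaps its Box, it applies a velocity-change impulse to the ball's Sphere, opposite the player's Arrow forward vector and scaled by Rebound.
; It then calls the player's TakeDamage with Damage and prints the returned value on screen.
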(event `self.Box.OnComponentBeginOverlap`
  (params (OverlappedComponent :type "PrimitiveComponent Object Reference") (OtherActor :type "Actor Object Reference") (OtherComp :type "PrimitiveComponent Object Reference") (OtherBodyIndex :type Integer) (bFromSweep :type Boolean) (SweepResult :type "HitResult Structure (by ref)"))
  (bind _asbp_ball_player (cast `/Game/RollingBall/Blueprint/Character/BP_BallPlayer` OtherActor))
  (`|ExecutionSequence`
    (:`then_0`
      ;[1 1 1] 進行方向の逆に力を与える
      (`PrimitiveComponent.AddImpulse` (`/Game/RollingBall/Blueprint/Character/BP_BallPlayer.Sphere` _asbp_ball_player) (* (`SceneComponent.GetForwardVector` (`/Game/RollingBall/Blueprint/Character/BP_BallPlayer.Arrow` _asbp_ball_player)) (* (`self.Rebound`) -1.0)) "None" true))
    (:`then_1`
      ;[1 1 1] PlayerにDamageを与える
      (bind _returnvalue (`/Game/RollingBall/Blueprint/Character/BP_BallPlayer.Take Damage` _asbp_ball_player (`self.Damage`)))
      (`KismetSystemLibrary.PrintString` (`KismetStringLibrary.Conv_DoubleToString` _returnvalue) true true (struct :`R` 1.0 :`B` 0.160625 :`A` 1.0) 10.0))))

(fn `UserConstructionScript`)